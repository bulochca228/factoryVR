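; Getter actor that takes in a resource of the type it needs through overlap.
; While not full, an overlapping resours_bp whose Type matches NeedType is destroyed.
; The overlap then sets IsFull to false, so pickup never marks the getter as full.
; A separate PickUpResours function also clears IsFull.
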(event `self.ReceiveActorBeginOverlap`
  (params (OtherActor :type "Actor Object Reference"))
  (if (not (`self.isFull`))
    (bind _asresours_bp (cast `/Game/actor/resours_bp` OtherActor))
    (if (`KismetStringLibrary.EqualEqual_StrStr` (`/Game/actor/resours_bp.Type` _asresours_bp) (`self.NeedType`))
      (`self.K2_DestroyActor` OtherActor)
      (set `self.isFull` false))))

(fn `Pick up resours`
  (set `self.isFull` false))

(fn `UserConstructionScript`)